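; Foods_BP is a physics food pickup that takes a random mesh and can be carried by the Doveman player or a PigBoss.
; On overlap, Doveman takes it when pressing grab empty-handed, while PigBoss takes it only if the first FoodTower's YesFood is set.
; Pickup disables physics and opens a Tick gate that snaps it to the carrier's Billboard.
; Drop/Taken restores collision and closes the gate, without re-enabling physics.
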(event OnComponentBeginOverlap(StaticMesh)
  (params (OverlappedComponent :type Primitive%20Component%20Object%20Reference) (OtherActor :type Actor%20Object%20Reference) (OtherComp :type Primitive%20Component%20Object%20Reference) (OtherBodyIndex :type Integer) (bFromSweep :type Boolean) (SweepResult :type Hit%20Result%20Structure%20%28by%20ref%29))
  (bind _outactors (Actor|GetAllActorsOfClass "/Game/_WhiteCollared/Mesh_Tester/PigBoss/FoodTower/FoodTower.FoodTower_C"))
  (if (Variables|/Game/_WhiteCollared/Mesh_Tester/PigBoss/FoodTower/FoodTower.FoodTower_C|GetYes%20Food (Utilities|Array|Get(acopy) _outactors))
    (bind _aspig_boss (Utilities|Casting|CastToPigBoss OtherActor))
    (Variables|Default|SetPigBoss%20Ref _aspig_boss)
    (Variables|Default|SetPig%20Has true)
    (CallFunction|Got)
    (else
      (Variables|Default|SetPig%20Has false)
      (bind _asdoveman (Utilities|Casting|CastToDoveman OtherActor))
      (Variables|Default|SetDoveman%20Ref _asdoveman)
      (if (and (Variables|/Game/_WhiteCollared/Mesh_Tester/Doveman.Doveman_C|GetGrab%20Pressed (Variables|Default|GetDoveman%20Ref)) (not (Variables|/Game/_WhiteCollared/Mesh_Tester/Doveman.Doveman_C|GetHas%20Item (Variables|Default|GetDoveman%20Ref))))
        (Variables|/Game/_WhiteCollared/Mesh_Tester/Doveman.Doveman_C|SetHas%20Item (Variables|Default|GetDoveman%20Ref) true)
        (Variables|/Game/_WhiteCollared/Mesh_Tester/Doveman.Doveman_C|SetGrab%20Pressed (Variables|Default|GetDoveman%20Ref) false)
        (CallFunction|Got)))))

(event Custom|Got
  (bind _doveman_ref (Variables|Default|GetDoveman%20Ref))
  (Physics|SetSimulatePhysics (Variables|Default|GetStaticMesh) false)
  (Collision|SetCollisionEnabled (Variables|Default|GetStaticMesh) "NoCollision")
  (Utilities|FlowControl|Gate true) ; enters at Open
)

(event Custom|Drop/Taken
  (bind _doveman_ref (Variables|Default|GetDoveman%20Ref))
  (Collision|SetCollisionEnabled (Variables|Default|GetStaticMesh) "QueryAndPhysics")
  (Utilities|FlowControl|Gate true) ; enters at Close
)

(event EventTick
  (params (DeltaSeconds :type Float%20%28single-precision%29))
  (bind _doveman_ref (Variables|Default|GetDoveman%20Ref))
  (Utilities|FlowControl|Gate true
    (:Exit
      (if (Variables|Default|GetPig%20Has)
        (Transformation|SetActorRelativeLocation (Transformation|GetWorldLocation (Variables|/Game/_WhiteCollared/Mesh_Tester/PigBoss/PigBoss.PigBoss_C|GetBillboard (Variables|Default|GetPigBoss%20Ref))))
        (elif (Variables|/Game/_WhiteCollared/Mesh_Tester/Doveman.Doveman_C|GetHas%20Item _doveman_ref)
          (Transformation|SetActorRelativeLocation (Transformation|GetWorldLocation (Variables|/Game/_WhiteCollared/Mesh_Tester/Doveman.Doveman_C|GetBillboard _doveman_ref)))
          (Transformation|SetActorRotation (Math|Conversions|RotationFromXVector (Math|Vector|GetForwardVector (Variables|/Script/Engine.Character|GetMesh _doveman_ref)))))))))

(event EventBeginPlay
  (bind _returnvalue (Math|Random|RandomIntegerinRange 0 2))
  (bind _asdoveman (Utilities|Casting|CastToDoveman (Game|GetPlayerCharacter 0)))
  (Variables|/Game/_WhiteCollared/Mesh_Tester/Doveman.Doveman_C|SetGone _asdoveman false)
  (Physics|SetSimulatePhysics (Variables|Default|GetStaticMesh) true)
  (Variables|Default|SetFood%20Mesh%20# _returnvalue)
  (Components|StaticMesh|SetStaticMesh (Variables|Default|GetStaticMesh) (Utilities|Array|Get(acopy) (Variables|Default|GetFood) _returnvalue)))

(fn ConstructionScript)